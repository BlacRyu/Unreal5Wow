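; RTS player controller that drives the camera pawn, issues move orders to selected units and offers a debug unit-spawn key.
; CameraTick pans via keys, curve-weighted edge scrolling or grip-drag in StarCraft 2 (normal/inverted) or Dota 2 style.
; Zoom sets spring arm length; scroll speed sets pawn MaxSpeed.
; Move orders reach each UnitController, queued or replacing, targeting a cursor ground trace that falls back to a camera-height plane.
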(event Custom|PrintAnalogValues
  ;[1 1 1] (DEBUG) Print analog stick values
)

(event EventTick
  (params (DeltaSeconds :type Float%20%28single-precision%29))
  (Utilities|FlowControl|Sequence
    (:then_0
      (CallFunction|CameraTick)
      (Variables|Default|SetbShowMouseCursor (CallFunction|ShouldCursorDisplay)))
    (:then_1
      (CallFunction|PrintAnalogValues))))

(event Input|ActionEvents|InputActionDebugSpawnUnit
  (params (Key :type Key%20Structure :default "None"))
  (bind (_location _success) (CallFunction|GetGroundUnderCursor))
  ;[1 1 1] (DEBUG) Spawn and select a unit
  (:Pressed
    (if _success
      (bind _returnvalue (AI|SpawnAIFromClass "/Game/RTS/Blueprints/Unit/Unit.Unit_C" 0 (+ _location "0,0,100.000000") (Math|Rotator|MakeRotator 0.0 0.0 (Math|Random|RandomFloat)) true 0))
      (Utilities|Array|AddUnique (Variables|Default|GetOwn%20Units) _returnvalue)
      (Utilities|Array|AddUnique (Variables|Default|GetOwn%20Selected%20Units) _returnvalue)
      (else
        (Development|PrintString "Failed to spawn test unit, couldn't find position under cursor")))))

(event Input|ActionEvents|InputActionQueueOrders
  (params (Key :type Key%20Structure))
  (:Pressed
    (Variables|Default|SetShouldQueueOrders true))
  (:Released
    (Variables|Default|SetShouldQueueOrders false)))

(event Input|ActionEvents|InputActionOrderStop
  (params (Key :type Key%20Structure)))

(event Input|ActionEvents|InputActionOrderMove
  (params (Key :type Key%20Structure))
  (bind _location (CallFunction|GetGroundUnderCursor))
  ;[1 1 1] Move selected units to target location
  (:Pressed
    (Utilities|FlowControl|Sequence
      (:then_0
        (for _array_element (Variables|Default|GetOwn%20Selected%20Units)
          (bind _asunit_controller (Utilities|Casting|CastToUnitController (Pawn|GetController _array_element)))
          (Default|Move _asunit_controller 0 _location false (select (Variables|Default|GetShouldQueueOrders) (Utilities|Enum|LiteralenumEOrderQueuePlacement "Back") (Utilities|Enum|LiteralenumEOrderQueuePlacement "ReplaceAll")))))
      (:then_1
        (Niagara|SpawnSystematLocation "/Game/Cursor/FX_Cursor.FX_Cursor" _location "0, 0, 0" "1.000000,1.000000,1.000000" true true "AutoRelease")))))

(event Custom|Camera%20Tick
  ;[1 1 1] Camera Grip
  (if (Variables|Camera|Grip|GetIs%20Gripping)
    (switch Utilities|FlowControl|Switch|SwitchonECameraGripStyle (Variables|Default|GetCamera%20Grip%20Style)
      (:NewEnumerator0
        (|Starcraft2stylegrip :!label _label))
      (:NewEnumerator1
        (goto _label Inverted))
      (:NewEnumerator2
        (|Dota2stylegrip)))
    (else
      ;[1 1 1] Camera Scroll hotkeys
      (Pawn|Input|AddMovementInput (Pawn|GetControlledPawn) (Math|Conversions|ToVector(Vector2D) (Class|KismetMathLibrary|GetRotated2D (Math|Vector2D|MakeVector2D (Input|AxisValues|GetScrollCameraDownUp) (Input|AxisValues|GetScrollCameraLeftRight)) (.Yaw (Math|Rotator|BreakRotator (Pawn|GetControlRotation :!class /Script/Engine.Controller))))) 1.0 false)
      ;[1 1 1] Edge Scroll
      (if (Math|Boolean|ANDBoolean (Variables|Camera|Scroll|GetEdge%20Scroll) (CallFunction|CursorIsonScreenEdge) (Class|UtilBlueprintFunctionLibrary|ViewportHasFocus))
        (Pawn|Input|AddMovementInput (Pawn|GetControlledPawn) (Math|Conversions|ToVector(Vector2D) (Class|KismetMathLibrary|GetRotated2D "(X=0.000000,Y=1.000000)" (.Yaw (Math|Rotator|BreakRotator (Pawn|GetControlRotation :!class /Script/Engine.Controller))))) (Math|Curves|GetFloatValue (Variables|Camera|Scroll|GetEdge%20Scroll%20Influence%20Curve) (* (- (/ (.LocationX (Game|Player|GetMousePosition)) (.SizeX (HUD|GetViewportSize))) 0.5) 2.0)) false)
        (Pawn|Input|AddMovementInput (Pawn|GetControlledPawn) (Math|Conversions|ToVector(Vector2D) (Class|KismetMathLibrary|GetRotated2D "(X=1.000000,Y=0.000000)" (.Yaw (Math|Rotator|BreakRotator (Pawn|GetControlRotation :!class /Script/Engine.Controller))))) (Math|Curves|GetFloatValue (Variables|Camera|Scroll|GetEdge%20Scroll%20Influence%20Curve) (* (- (/ (.LocationY (Game|Player|GetMousePosition)) (.SizeY (HUD|GetViewportSize))) 0.5) -2.0)) false)))))

(event EventPossess
  (params (PossessedPawn :type Pawn%20Object%20Reference))
  ;[1 1 1] Initialize camera speed
  (CallFunction|SetScrollSpeed (Variables|Camera|Scroll|GetDefault%20Scroll%20Speed))
  ;[1 1 1] Initialize camera zoom
  (CallFunction|SetZoom (Variables|Camera|Zoom|GetDefault%20Zoom)))

(event Input|ActionEvents|InputActionZoomCameraIn
  (params (Key :type Key%20Structure))
  ;[1 1 1] Camera Zoom hotkeys
  (:Pressed
    (CallFunction|ZoomCamera (* (Variables|Camera|Zoom|GetZoom%20Increment) -1.0))))

(event Input|ActionEvents|InputActionCameraGrip
  (params (Key :type Key%20Structure))
  (bind (_locationx _locationy) (Game|Player|GetMousePosition))
  ;[1 1 1] Camera Grip
  ;;[1 1 1] Capture state when button is pressed
  (:Pressed
    (Variables|Camera|Grip|SetIs%20Gripping true)
    (Variables|Camera|Grip|SetGrip%20World%20Location (.Location (Collision|BreakHitResult (.HitResult (Game|Player|GetHitResultUnderCursorbyChannel "TraceTypeQuery1" true)))))
    (Variables|Camera|Grip|SetGrip%20Screen%20Position (Math|Vector2D|MakeVector2D _locationx _locationy))
    (Variables|Camera|Grip|SetGrip%20Camera%20Location (Transformation|GetActorLocation (Pawn|GetControlledPawn))))
  (:Released
    (Variables|Camera|Grip|SetIs%20Gripping false)))

(event Input|ActionEvents|InputActionZoomCameraOut
  (params (Key :type Key%20Structure))
  ;[1 1 1] Camera Zoom hotkeys
  (:Pressed
    (CallFunction|ZoomCamera (Variables|Camera|Zoom|GetZoom%20Increment))))

(fn ConstructionScript)

(fn GetGroundUnderCursor
  (bind (_worldlocation _worlddirection) (Game|Player|ConvertMouseLocationToWorldSpace))
  (bind _hitresult (Game|Player|GetHitResultUnderCursorbyChannel "TraceTypeQuery3" true))
  (bind _returnvalue (Pawn|GetControlledPawn))
  (bind (_bblockinghit _binitialoverlap _time _distance _location) (Collision|BreakHitResult _hitresult))
  (bind _returnvalue_2 (Transformation|GetActorLocation _returnvalue))
  (bind _returnvalue_3 (+ _worldlocation _worlddirection))
  (bind (_t _intersection _returnvalue_4) (Class|KismetMathLibrary|LinePlaneIntersectionOriginNormal _worldlocation _returnvalue_3 _returnvalue_2 "0, 0,1.000000"))
  (if _bblockinghit
    (LocalVariables|SetHit%20Location _location)
    (LocalVariables|SetSuccessful%20Hit _bblockinghit)
    (else
      ;[1 1 1] If there is no ground collision under the cursor, check against a plane extending from the camera's focus position
      (LocalVariables|SetHit%20Location _intersection)
      (LocalVariables|SetSuccessful%20Hit _returnvalue_4)))
  (return (LocalVariables|GetHit%20Location) (LocalVariables|GetSuccessful%20Hit)))

(fn ZoomCamera
  (params (Amount :type Float%20%28double-precision%29))
  (CallFunction|SetZoom (+ Amount (CallFunction|GetZoom)))
  (return))

(fn SetZoom
  (params (NewZoom :type Float%20%28single-precision%29))
  (bind _output_get (Variables|/Script/Engine.SpringArmComponent|SetTargetArmLength (CallFunction|GetSpringArm) (Math|Float|Clamp(Float) NewZoom (Variables|Camera|Zoom|GetMin%20Zoom) (Variables|Camera|Zoom|GetMax%20Zoom))))
  (return _output_get))

(fn GetZoom
  (return (Variables|/Script/Engine.SpringArmComponent|GetTargetArmLength (CallFunction|GetSpringArm))))

(fn SetScrollSpeed
  (params (New%20Speed :type Float%20%28single-precision%29))
  (bind _asfloating_pawn_movement (Utilities|Casting|CastToFloatingPawnMovement (Pawn|GetMovementComponent (Pawn|GetControlledPawn))))
  (Variables|/Script/Engine.FloatingPawnMovement|SetMaxSpeed _asfloating_pawn_movement New%20Speed))

(fn GetScrollSpeed
  (bind _asfloating_pawn_movement (Utilities|Casting|CastToFloatingPawnMovement (Pawn|GetMovementComponent (Pawn|GetControlledPawn))))
  (return (Class|MovementComponent|GetMaxSpeed _asfloating_pawn_movement)))

(fn GetSpringArm
  (return (Actor|GetComponentbyClass (Pawn|GetControlledPawn) "/Script/Engine.SpringArmComponent")))

(fn GetCamera
  (return (Actor|GetComponentbyClass (Pawn|GetControlledPawn) "/Script/Engine.CameraComponent")))

(fn ShouldCursorDisplay
  (return (or (Variables|Default|GetAlways%20Show%20Cursor) (|HideduringSC2stylecameragrip))))

(fn CursorIsonScreenEdge
  (bind (_locationx _locationy _returnvalue) (Game|Player|GetMousePosition))
  (bind (_sizex _sizey) (HUD|GetViewportSize))
  (if _returnvalue
    (LocalVariables|SetMouse%20X _locationx)
    (LocalVariables|SetMouse%20Y _locationy)
    (LocalVariables|SetViewport%20X _sizex)
    (LocalVariables|SetViewport%20Y _sizey)
    (return (and (Math|Boolean|ANDBoolean (>= (LocalVariables|GetMouse%20X) 0.0) (<= (LocalVariables|GetMouse%20X) (LocalVariables|GetViewport%20X)) (>= (LocalVariables|GetMouse%20Y) 0.0) (<= (LocalVariables|GetMouse%20Y) (LocalVariables|GetViewport%20Y))) (Math|Boolean|ORBoolean (<= (LocalVariables|GetMouse%20X) (Variables|Camera|Scroll|GetEdge%20Scroll%20Distance)) (>= (LocalVariables|GetMouse%20X) (- (LocalVariables|GetViewport%20X) (Variables|Camera|Scroll|GetEdge%20Scroll%20Distance))) (<= (LocalVariables|GetMouse%20Y) (Variables|Camera|Scroll|GetEdge%20Scroll%20Distance)) (>= (LocalVariables|GetMouse%20Y) (- (LocalVariables|GetViewport%20Y) (Variables|Camera|Scroll|GetEdge%20Scroll%20Distance))))))
    (else
      ;[1 1 1] Invalid mouse position
      (return false))))