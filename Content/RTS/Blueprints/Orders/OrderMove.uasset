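; OrderMove is an RTS move order that sends a controlled unit to a target unit or a fixed position.
; Init stores its parameters and returns self; on begin, it runs an AIMoveTo task through the UnitController, favoring a valid target unit over the position.
; Either finish or request failure marks the order completed, while interruption stops movement.
; DirectPathing is stored but unused in these graphs, and IsUnitMoving checks controller move status.
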(event EventOnBegin
  (bind _asunit_controller (Utilities|Casting|CastToUnitController (Pawn|GetController (Variables|Default|Get_ControlledUnit))))
  (bind _asynctaskproxy (AI|AIMoveTo _asunit_controller (CallFunction|GetTargetLocation) (Variables|Default|Get_TargetUnit) -1.0 "Default" "Default" true false)
    (:then
      (Variables|Default|SetMoveAsyncTask _asynctaskproxy))
    (:OnRequestFailed
      (Variables|Default|SetbCompleted true :!label _label))
    (:OnMoveFinished
      (goto _label))))

(event EventOnInterrupted
  (AI|Navigation|StopMovement (Pawn|GetController (Variables|Default|Get_ControlledUnit))))

(fn Init
  (params (ControlledUnit :type Unit%20Object%20Reference) (TargetUnit :type Unit%20Object%20Reference) (TargetPosition :type Vector) (DirectPathing :type Boolean))
  (Utilities|FlowControl|Sequence
    (:then_0
      (Variables|Default|Set_ControlledUnit ControlledUnit))
    (:then_1
      (Variables|Default|Set_TargetUnit TargetUnit))
    (:then_2
      (Variables|Default|Set_TargetPosition TargetPosition))
    (:then_3
      (Variables|Default|SetDirect%20Pathing DirectPathing))
    (:then_4
      (return self))))

(fn GetTargetLocation
  (bind __targetunit (Variables|Default|Get_TargetUnit))
  (Utilities|IsValid __targetunit
    (:Is%20Valid
      (return (Transformation|GetActorLocation __targetunit)))
    (:Is%20Not%20Valid
      (return (Variables|Default|Get_TargetPosition)))))