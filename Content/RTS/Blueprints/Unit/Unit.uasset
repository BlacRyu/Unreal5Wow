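; Base RTS unit actor with a selection circle, toggled by Selected and Unselected events, and simple crowd avoidance.
; Each tick it adds a constant downward velocity to its FloatingPawnMovement, then pushes itself away from overlapping units.
; Overlap events maintain the neighbor list, and a falloff curve over distance relative to the avoidance sphere radius scales each push.
; Helpers provide edge and center distances, plus a healthbar debug printout.
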(event Custom|Unselected
  (Rendering|SetVisibility (Variables|Default|GetSelection%20Circle) false false))

(event Custom|Selected
  (Rendering|SetVisibility (Variables|Default|GetSelection%20Circle) true false))

(event EventTick
  (params (DeltaSeconds :type Float%20%28single-precision%29))
  (Utilities|FlowControl|Sequence
    (:then_0
      (Utilities|ApplyGravity))
    (:then_1
      (Utilities|Avoidance))))

(event Collision|EventActorBeginOverlap
  (params (OtherActor :type Actor%20Object%20Reference))
  (bind _asunit (Utilities|Casting|CastToUnit OtherActor))
  (Utilities|Array|AddUnique (Variables|Default|GetOverlapping%20Units) _asunit))

(event Collision|EventActorEndOverlap
  (params (OtherActor :type Actor%20Object%20Reference))
  (bind _asunit (Utilities|Casting|CastToUnit OtherActor))
  (Utilities|Array|RemoveItem (Variables|Default|GetOverlapping%20Units) _asunit))

(fn ConstructionScript)

(fn EdgetoEdgeDistance
  (params (Other%20Unit :type Unit%20Object%20Reference))
  (return (Utilities|Operators|Subtract (Transformation|GetDistanceTo Other%20Unit) (Components|Capsule|GetScaledCapsuleRadius (Variables|Unit_C|GetCapsule Other%20Unit)) (Components|Capsule|GetScaledCapsuleRadius (Variables|Default|GetCapsule)))))

(fn CentertoCenterDistance
  (params (Other%20Unit :type Unit%20Object%20Reference))
  (return (Transformation|GetDistanceTo Other%20Unit)))